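; BP_GhostTrail is an afterimage actor that shows a frozen copy of the player's third-person pose.
; On BeginPlay it gives each poseable mesh material slot a dynamic M_GhostTrail instance, copies the player's pose and starts an opacity timeline.
; The timeline's handlers, marked as never run, would push opacity to those materials (parameter name unset) and destroy the actor on finish.
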(event Custom|GhostTrail
  (for _array_element (Rendering|Material|GetMaterials (Variables|Default|GetPoseableMesh))
    (bind _returnvalue (Rendering|Material|CreateDynamicMaterialInstance "/Game/Blueprints/TESTS/M_GhostTrail.M_GhostTrail" "None" "None" :!class /Script/Engine.KismetMaterialLibrary))
    (bind _returnvalue_2 (Utilities|Array|Add (Variables|Default|GetDynamicMats) _returnvalue))
    (Rendering|Material|SetMaterial (Variables|Default|GetPoseableMesh) _returnvalue_2 _returnvalue)
    (Class|PoseableMeshComponent|CopyPosefromSkeletalComponent (Variables|Default|GetPoseableMesh) (Variables|/Game/Blueprints/Player/BP_PlayerCharacter.BP_PlayerCharacter_C|GetThirdPersonMesh (Variables|Default|GetAs%20BP%20Player%20Character)))
    (Components|Timeline|PlayfromStart (Variables|Default|GetOpacityTimeline))))

(event EventBeginPlay
  (bind _asbp_player_character (Utilities|Casting|CastToBP_PlayerCharacter (Game|Player|GetPlayerPawn 0)))
  (Variables|Default|SetAs%20BP%20Player%20Character _asbp_player_character)
  (CallFunction|GhostTrail))

(fn ConstructionScript
  (Utilities|Array|Clear (Variables|Default|GetDynamicMats)))