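; GA_DashAbility is the player's dash gameplay ability, currently a stub that performs no movement.
; On activation it caches the BP_PlayerCharacter pawn, prints a debug "Ethereal" message and ends immediately.
; Disconnected legacy "Ethereal" dash nodes remain: a movement-state switch, a BP_CableLink from the player's pelvis to a shadow mesh, a delay, and separate cleanup restoring walking.
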(event Ability|EventActivateAbility
  (bind _output_get (Utilities|GetPlayerCharacter))
  (Development|PrintString "Ethereal")
  (Ability|EndAbility))

(event Ability|EventOnEndAbility
  (params (bWasCancelled :type Boolean)))