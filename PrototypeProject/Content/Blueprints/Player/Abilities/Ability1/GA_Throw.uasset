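; GA_Throw is a player Gameplay Ability that throws a projectile in two stages.
; Activation calls StartFiringProj on the combat component, then waits for an input press to call ShootProjectile, print a debug message and end the ability.
; A helper gets MACCombatComponent from player pawn 0 rather than the ability's actor info, so it assumes the local first player.
; Montage and gameplay-event wait nodes are left unconnected.
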(event Ability|EventActivateAbility
  (bind _m_accombatcomponent (Utilities|GetCombatComponent))
  (Class|CombatComponent|StartFiringProj _m_accombatcomponent)
  (Ability|Tasks|WaitInputPress false
    (:OnPress
      (bind _m_accombatcomponent_2 (Utilities|GetCombatComponent))
      (Class|CombatComponent|ShootProjectile _m_accombatcomponent_2)
      (Development|PrintString "Threw")
      (Ability|EndAbility))))

(event Ability|EventOnEndAbility
  (params (bWasCancelled :type Boolean)))